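; Pistol child of a base gun class that fires one BP_Bullet per Fire call and tracks its ammo.
; Setup creates the pistol widget and has the player controller display it.
; Fire passes a check fed by the aiming state, then spawns a damage-carrying bullet at ShootSocket, rotated toward the camera trace's end point rather than its impact.
; Reload refills ammo to maximum, and Tick prints the count for debugging.
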(event Custom|DecrementCurrentAmmo
  ;[1 1 1] Decrement Current Ammo
  (Variables|Default|SetCurrent%20Ammo (- (Variables|Default|GetCurrent%20Ammo) 1)))

(event EventBeginPlay
  (|CallParentFunction) ; This node is disabled and will not be called.\nDrag off pins to build functionality.
)

(event Collision|EventActorBeginOverlap
  (params (OtherActor :type Actor%20Object%20Reference))
  (|CallParentFunction OtherActor) ; This node is disabled and will not be called.\nDrag off pins to build functionality.
)

(event EventReload
  ;[1 1 1] Reload Firearm with Max Ammo Value
  (Variables|Default|SetCurrent%20Ammo (Variables|Default|GetMax%20Ammo))
  (|CallParentFunction))

(event EventFire
  (bind _skeletalmesh (Variables|Default|GetSkeletalMesh))
  (bind _returnvalue (Transformation|GetSocketLocation _skeletalmesh "ShootSocket"))
  ;[1 1 1] Fires Single Bullet Per Click
  (bind _asbp_first_person_character (Utilities|Casting|CastToBP_FirstPersonCharacter (Game|GetPlayerCharacter 0)))
  (bind _valid (CallFunction|Checkers (Variables|/Game/FirstPerson/Blueprints/BP_FirstPersonCharacter.BP_FirstPersonCharacter_C|GetisAiming _asbp_first_person_character)))
  (if _valid
    ;;[1 1 1] Bullet is spawned from the Pistol's ShootSocket, and is aimed at where the player's camera is looking.
    (bind _outhit (Collision|LineTraceByChannel (Transformation|GetWorldLocation (Variables|/Game/FirstPerson/Blueprints/BP_FirstPersonCharacter.BP_FirstPersonCharacter_C|GetFirstPersonCamera _asbp_first_person_character)) (+ (Transformation|GetWorldLocation (Variables|/Game/FirstPerson/Blueprints/BP_FirstPersonCharacter.BP_FirstPersonCharacter_C|GetFirstPersonCamera _asbp_first_person_character)) (* (Math|Vector|GetForwardVector (Variables|/Game/FirstPerson/Blueprints/BP_FirstPersonCharacter.BP_FirstPersonCharacter_C|GetFirstPersonCamera _asbp_first_person_character)) 5e+03)) "TraceTypeQuery1" false 0 "None"))
    (Game|SpawnActorfromClass "/Game/ProgressionProject/Blueprints/BP_Bullet.BP_Bullet_C" (Math|Transform|MakeTransform _returnvalue (Math|Rotator|FindLookatRotation _returnvalue (.TraceEnd (Collision|BreakHitResult _outhit)))) "AlwaysSpawn" "MultiplyWithRoot" 0 (Variables|Default|GetDMG) 0)
    (CallFunction|DecrementCurrentAmmo)
    (|CallParentFunction)))

(event EventTick
  (params (DeltaSeconds :type Float%20%28single-precision%29))
  (Development|PrintString (Utilities|String|ToString(Text) (Utilities|Text|FormatText "Found in BP_Pistol: 
Current Ammo: {x}" (Variables|Default|GetCurrent%20Ammo))) true true "(R=0.000000,G=0.660000,B=1.000000,A=1.000000)" (Utilities|Time|GetWorldDeltaSeconds)))

(event EventBaseGunSetup
  (bind _returnvalue (Game|GetPlayerController 0))
  ;[1 1 1] On Collision and after Firearm is attached to the Player, set Pistol Widget to Gun Widget and Display to Player.
  (|CallParentFunction)
  (bind _returnvalue_2 (UserInterface|CreateWidget "/Game/ProgressionProject/Blueprints/Widget_Blueprints/WBP_Pistol.WBP_Pistol_C" _returnvalue))
  (Variables|Default|SetGunWidget _returnvalue_2)
  (bind _asbp_first_person_player_controller (Utilities|Casting|CastToBP_FirstPersonPlayerController _returnvalue))
  (Default|DisplayGunWidget _asbp_first_person_player_controller))

(fn ConstructionScript
  (|CallParentFunction))
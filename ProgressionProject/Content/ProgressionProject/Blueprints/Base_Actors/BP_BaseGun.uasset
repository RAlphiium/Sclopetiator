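; BP_BaseGun is the base gun actor that the first-person character picks up by walking into its sphere.
; On overlap it casts to BP_FirstPersonCharacter, stores that reference, sets itself as the character's CurrentGun and calls AttachGun.
; Fire and Reload are placeholder events that only print, left for derived guns to implement.
; The Checkers function returns true only when aiming with ammo remaining, though nothing here calls it.
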(event OnComponentBeginOverlap(Sphere)
  (params (OverlappedComponent :type Primitive%20Component%20Object%20Reference) (OtherActor :type Actor%20Object%20Reference) (OtherComp :type Primitive%20Component%20Object%20Reference) (OtherBodyIndex :type Integer) (bFromSweep :type Boolean) (SweepResult :type Hit%20Result%20Structure%20%28by%20ref%29))
  ;[1 1 1] Writes the Player Character's Current Weapon attribute as this actor's self and runs the First Person Character's AttachWeapon Event.
  (bind _asbp_first_person_character (Utilities|Casting|CastToBP_FirstPersonCharacter OtherActor))
  (Variables|Default|SetAs%20BP%20First%20Person%20Character _asbp_first_person_character)
  (CallFunction|BaseGunSetup))

(event Custom|BaseGun%20Setup
  (bind _as_bp_first_person_character (Variables|Default|GetAs%20BP%20First%20Person%20Character))
  ;[1 1 1] Writes the Player Character's Current Weapon attribute as this actor's self and runs the First Person Character's AttachWeapon Event.
  (Variables|/Game/FirstPerson/Blueprints/BP_FirstPersonCharacter.BP_FirstPersonCharacter_C|SetCurrentGun _as_bp_first_person_character self)
  (Default|AttachGun _as_bp_first_person_character))

(event Custom|Fire
  ;[1 1 1] Event that Derived Actors can access. Will need to enable Gun Actors to shoot.
  (Development|PrintString "Fire"))

(event Custom|Reload
  ;[1 1 1] Event that Derived Actors can access. Will need to enable Gun Actors to shoot.
  (Development|PrintString "Reload."))

(event EventBeginPlay
  (|CallParentFunction) ; This node is disabled and will not be called.\nDrag off pins to build functionality.
)

(event Collision|EventActorBeginOverlap
  (params (OtherActor :type Actor%20Object%20Reference))
  (|CallParentFunction OtherActor) ; This node is disabled and will not be called.\nDrag off pins to build functionality.
)

(event EventTick
  (params (DeltaSeconds :type Float%20%28single-precision%29))
  (|CallParentFunction DeltaSeconds) ; This node is disabled and will not be called.\nDrag off pins to build functionality.
)

(fn ConstructionScript
  (|CallParentFunction))

(fn Checkers
  (params (isAiming :type Boolean))
  (if (== isAiming true)
    (if (> (Variables|Default|GetCurrent%20Ammo) 0)
      (return true)
      (else
        _)))
  (return false))
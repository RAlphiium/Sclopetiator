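; BP_WaveChecker tracks the total number of living enemies across all spawners and advances the wave count when none remain.
; On BeginPlay it binds to dispatchers that add each spawner's count and decrement the total per eliminated enemy.
; When the total reaches zero it increments WaveNumber and only prints a "Spawn New Enemies" message.
; Tick prints the current enemy count as on-screen debug text.
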(event Custom|Eon_CalculateTotalEnemies_Event
  (params (TotalFromSpawner :type Integer))
  ;[1 1 1] Calculates Total From All Spawners
  (Variables|Default|SetTotalEnemies (+ TotalFromSpawner (Variables|Default|GetTotalEnemies))))

(event Custom|Eon_DecrementTotalEnemies_Event
  ;[1 1 1] When Enemy is eliminated, call Event Dispatcher and decrement TotalEnemies.
  (bind _output_get (Variables|Default|SetTotalEnemies (- (Variables|Default|GetTotalEnemies) 1)))
  (if (== _output_get 0)
    (Variables|Default|SetWaveNumber (+ 1 (Variables|Default|GetWaveNumber)))
    (Development|PrintString "Spawn New Enemies")))

(event EventBeginPlay
  ;[1 1 1] Bind Event Dispatcher
  (EventDispatchers|BindEventtoEonCalculateTotalEnemies (EventDispatchers|CreateEvent :!event Custom|Eon_CalculateTotalEnemies_Event))
  (EventDispatchers|BindEventtoEonDecrementTotalEnemies (EventDispatchers|CreateEvent :!event Custom|Eon_DecrementTotalEnemies_Event)))

(event EventTick
  (params (DeltaSeconds :type Float%20%28single-precision%29))
  (Development|PrintString (Utilities|String|ToString(Text) (Utilities|Text|FormatText "Found in WaveChecker: 
Number of Enemies: {x}" (Utilities|String|ToString(Integer) (Variables|Default|GetTotalEnemies)))) true true "(R=0.000000,G=0.660000,B=1.000000,A=1.000000)" (Utilities|Time|GetWorldDeltaSeconds)))

(fn ConstructionScript)
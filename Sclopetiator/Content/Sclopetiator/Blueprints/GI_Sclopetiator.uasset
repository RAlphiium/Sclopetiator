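; Game instance for Sclopetiator that pushes centrally stored weapon stats onto the pistols and shotguns in the world.
; RewriteStats calls its parent version, then runs an update event for each weapon type.
; Each update finds all BP_Pistol or BP_Shotgun actors and overwrites their damage and reload speed from the matching PistolStats or ShotgunStats.
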(event Custom|UpdatePistols
  (bind _pistolstats (Variables|Default|GetPistolStats))
  (bind _outactors (Actor|GetAllActorsOfClass "/Game/Sclopetiator/Blueprints/BP_Pistol.BP_Pistol_C"))
  (for _array_element _outactors
    (Variables|/Game/Sclopetiator/Blueprints/Base_Actors/BP_BaseGun.BP_BaseGun_C|SetDMG _array_element (.dmg _pistolstats))
    (Variables|/Game/Sclopetiator/Blueprints/Base_Actors/BP_BaseGun.BP_BaseGun_C|SetReload%20Speed _array_element (.reloadspeed _pistolstats))))

(event Custom|UpdateShotguns
  (bind _shotgunstats (Variables|Default|GetShotgunStats))
  (bind _outactors (Actor|GetAllActorsOfClass "/Game/Sclopetiator/Blueprints/BP_Shotgun.BP_Shotgun_C"))
  (for _array_element _outactors
    (Variables|/Game/Sclopetiator/Blueprints/Base_Actors/BP_BaseGun.BP_BaseGun_C|SetDMG _array_element (.dmg _shotgunstats))
    (Variables|/Game/Sclopetiator/Blueprints/Base_Actors/BP_BaseGun.BP_BaseGun_C|SetReload%20Speed _array_element (.reloadspeed _shotgunstats))))

(event EventRewriteStats
  (|CallParentFunction)
  (CallFunction|UpdatePistols)
  (CallFunction|UpdateShotguns))
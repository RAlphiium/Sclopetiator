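; Melee enemy that knocks back and damages the first-person player on contact.
; When its Box overlaps an actor of exactly BP_FirstPersonCharacter class, it adds a velocity-change impulse to player 0 along the mesh's forward vector with an upward bias.
; It then casts PlayerTarget to that character and passes DMG to HealthModified.
; No movement or AI logic lives in this Blueprint's graphs.
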(event OnComponentBeginOverlap(Box)
  (params (OverlappedComponent :type Primitive%20Component%20Object%20Reference) (OtherActor :type Actor%20Object%20Reference) (OtherComp :type Primitive%20Component%20Object%20Reference) (OtherBodyIndex :type Integer) (bFromSweep :type Boolean) (SweepResult :type Hit%20Result%20Structure%20%28by%20ref%29))
  ;[1 1 1] Enemy - Player Collision
  (if (== (Utilities|GetClass OtherActor) "/Game/FirstPerson/Blueprints/BP_FirstPersonCharacter.BP_FirstPersonCharacter_C")
    (Physics|AddImpulse (Variables|/Script/Engine.Character|GetCharacterMovement (Game|GetPlayerCharacter 0)) (* (+ (Math|Vector|GetForwardVector (Variables|Default|GetStaticMesh)) "0.000000,0.000000,0.500000") 6e+02) true)
    (bind _asbp_first_person_character (Utilities|Casting|CastToBP_FirstPersonCharacter (Variables|Default|GetPlayerTarget)))
    (Class|SclopetiatorCharacter|HealthModified _asbp_first_person_character (Variables|Default|GetDMG))))

(event EventBeginPlay
  (|CallParentFunction) ; This node is disabled and will not be called.\nDrag off pins to build functionality.
)

(event Collision|EventActorBeginOverlap
  (params (OtherActor :type Actor%20Object%20Reference)))

(event EventTick
  (params (DeltaSeconds :type Float%20%28single-precision%29))
  (|CallParentFunction DeltaSeconds) ; This node is disabled and will not be called.\nDrag off pins to build functionality.
)

(fn ConstructionScript
  (|CallParentFunction))
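; Player projectile that damages melee and ranged enemies on overlap and awards score to the first-person character.
; Its box checks the enemy's Head, then Body, applying the same DMG to either, with headshots worth double the base points.
; A multiplier scales the points up as player health drops.
; The projectile destroys itself after the enemy check to prevent piercing.
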(event OnComponentBeginOverlap(Box)
  (params (OverlappedComponent :type Primitive%20Component%20Object%20Reference) (OtherActor :type Actor%20Object%20Reference) (OtherComp :type Primitive%20Component%20Object%20Reference) (OtherBodyIndex :type Integer) (bFromSweep :type Boolean) (SweepResult :type Hit%20Result%20Structure%20%28by%20ref%29))
  (bind _returnvalue (Utilities|GetClass OtherActor))
  ;[1 1 1] Bullet Collision
  (if (or (== _returnvalue "/Game/Sclopetiator/Blueprints/BP_NewMeleeEnemy.BP_NewMeleeEnemy_C") (== _returnvalue "/Game/Sclopetiator/Blueprints/BP_NewRangedEnemy.BP_NewRangedEnemy_C"))
    (bind _asbp_new_base_enemy (Utilities|Casting|CastToBP_NewBaseEnemy OtherActor))
    (CallFunction|CheckHead _asbp_new_base_enemy)
    ;;[1 1 1] Prevents Piercing Effect
    (Actor|DestroyActor)))

(event Custom|CheckHead
  (params (Enemy :type BP%20New%20Base%20Enemy%20Object%20Reference))
  ;[1 1 1] Checks if Head Component of Enemy has been Overlapped.
  (if (Class|PrimitiveComponent|IsOverlappingComponent (Variables|Default|GetBox) (Variables|/Game/Sclopetiator/Blueprints/Base_Actors/BP_NewBaseEnemy.BP_NewBaseEnemy_C|GetHead Enemy))
    (Default|DecrementHealth Enemy (Variables|Default|GetDMG))
    (bind _asbp_first_person_character (Utilities|Casting|CastToBP_FirstPersonCharacter (Game|GetPlayerCharacter 0)))
    (bind _multiplier (CallFunction|Multiplier (Variables|/Script/Sclopetiator.SclopetiatorCharacter|GetHealth _asbp_first_person_character)))
    (Class|SclopetiatorCharacter|ScorePointsModified _asbp_first_person_character (* _multiplier 50))
    (else
      (CallFunction|CheckBody Enemy))))

(event Custom|CheckBody
  (params (Enemy :type BP%20New%20Base%20Enemy%20Object%20Reference))
  ;[1 1 1] Checks if Body Component of Enemy has been Overlapped.
  (if (Class|PrimitiveComponent|IsOverlappingComponent (Variables|Default|GetBox) (Variables|/Game/Sclopetiator/Blueprints/Base_Actors/BP_NewBaseEnemy.BP_NewBaseEnemy_C|GetBody Enemy))
    (Default|DecrementHealth Enemy (Variables|Default|GetDMG))
    (bind _asbp_first_person_character (Utilities|Casting|CastToBP_FirstPersonCharacter (Game|GetPlayerCharacter 0)))
    (bind _multiplier (CallFunction|Multiplier (Variables|/Script/Sclopetiator.SclopetiatorCharacter|GetHealth _asbp_first_person_character)))
    (Class|SclopetiatorCharacter|ScorePointsModified _asbp_first_person_character (* _multiplier 25))))

(fn ConstructionScript
  (|CallParentFunction))

(fn Multiplier
  (params (Health :type Integer))
  (switch int Health
    (:Default
      (Development|PrintString "Not Posible; "))
    (:0
      (Development|PrintString "Not Posible; "))
    (:1
      (return 5))
    (:2
      (return 4))
    (:3
      (return 3))
    (:4
      (return 2))
    (:5
      (return 1)))
  (return 0))
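; Game instance for Sclopetiator's progression, holding stat points plus player, pistol, shotgun and rifle stats.
; Increment and decrement events edit pending MOD copies of stat points and player health, speed and luck in fixed steps, without internal bounds checks.
; RewriteStats copies all pending values into the live stats on confirmation.
; Separate helper functions report whether points remain, whether health and point totals are within limits, and whether two values differ.
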(event Custom|DecreasePlayerLuck
  ;[1 1 1] Decrease Player Luck
  (Variables|Default|SetMODPlayerStats (Utilities|Struct|MakeS_PlayerStats (.MaxHealth (Utilities|Struct|BreakS_PlayerStats (Variables|Default|GetMODPlayerStats))) (.Speed (Utilities|Struct|BreakS_PlayerStats (Variables|Default|GetMODPlayerStats))) (- (.Luck (Utilities|Struct|BreakS_PlayerStats (Variables|Default|GetMODPlayerStats))) 5.0))))

(event Custom|RewriteStats
  ;[1 1 1] Update Stats with Modified Stats after Confirmation
  (Variables|Default|SetStatPoints (Variables|Default|GetMODStatPoints))
  (Variables|Default|SetPlayerStats (Variables|Default|GetMODPlayerStats))
  (Variables|Default|SetPistolStats (Variables|Default|GetMODPistolStats))
  (Variables|Default|SetShotgunStats (Variables|Default|GetMODShotgunStats))
  (Variables|Default|SetRifleStats (Variables|Default|GetMODRifleStats)))

(event Custom|DecrementStatPoints
  ;[1 1 1] Decrement Stat Points
  (Variables|Default|SetMODStatPoints (- (Variables|Default|GetMODStatPoints) 1)))

(event Custom|IncrementStatPoints
  ;[1 1 1] Increment Stat Points
  (Variables|Default|SetMODStatPoints (+ (Variables|Default|GetMODStatPoints) 1)))

(event Custom|IncrementPlayerHealth
  ;[1 1 1] Increment Player Health
  (Variables|Default|SetMODPlayerStats (Utilities|Struct|MakeS_PlayerStats (+ (.MaxHealth (Utilities|Struct|BreakS_PlayerStats (Variables|Default|GetMODPlayerStats))) 1) (.Speed (Utilities|Struct|BreakS_PlayerStats (Variables|Default|GetMODPlayerStats))) (.Luck (Utilities|Struct|BreakS_PlayerStats (Variables|Default|GetMODPlayerStats))))))

(event Custom|DecrementPlayerHealth
  ;[1 1 1] Decrement Player Health
  (Variables|Default|SetMODPlayerStats (Utilities|Struct|MakeS_PlayerStats (- (.MaxHealth (Utilities|Struct|BreakS_PlayerStats (Variables|Default|GetMODPlayerStats))) 1) (.Speed (Utilities|Struct|BreakS_PlayerStats (Variables|Default|GetMODPlayerStats))) (.Luck (Utilities|Struct|BreakS_PlayerStats (Variables|Default|GetMODPlayerStats))))))

(event Custom|IncreasePlayerMovement
  ;[1 1 1] Increase Player Movement
  (Variables|Default|SetMODPlayerStats (Utilities|Struct|MakeS_PlayerStats (.MaxHealth (Utilities|Struct|BreakS_PlayerStats (Variables|Default|GetMODPlayerStats))) (+ (.Speed (Utilities|Struct|BreakS_PlayerStats (Variables|Default|GetMODPlayerStats))) 1e+02) (.Luck (Utilities|Struct|BreakS_PlayerStats (Variables|Default|GetMODPlayerStats))))))

(event Custom|DecreasePlayerMovement
  ;[1 1 1] Increase Player Movement
  (Variables|Default|SetMODPlayerStats (Utilities|Struct|MakeS_PlayerStats (.MaxHealth (Utilities|Struct|BreakS_PlayerStats (Variables|Default|GetMODPlayerStats))) (- (.Speed (Utilities|Struct|BreakS_PlayerStats (Variables|Default|GetMODPlayerStats))) 1e+02) (.Luck (Utilities|Struct|BreakS_PlayerStats (Variables|Default|GetMODPlayerStats))))))

(event Custom|IncreasePlayerLuck
  ;[1 1 1] Increase Player Luck
  (Variables|Default|SetMODPlayerStats (Utilities|Struct|MakeS_PlayerStats (.MaxHealth (Utilities|Struct|BreakS_PlayerStats (Variables|Default|GetMODPlayerStats))) (.Speed (Utilities|Struct|BreakS_PlayerStats (Variables|Default|GetMODPlayerStats))) (+ (.Luck (Utilities|Struct|BreakS_PlayerStats (Variables|Default|GetMODPlayerStats))) 5.0))))

(fn CheckStatPoints
  (if (> (Variables|Default|GetMODStatPoints) 0)
    (return true)
    (else
      (return false))))

(fn IsHealthValid
  (bind _modplayerstats (Variables|Default|GetMODPlayerStats))
  (bind _maxhealth (Utilities|Struct|BreakS_PlayerStats _modplayerstats))
  (if (or (>= _maxhealth 5) (<= _maxhealth 0))
    (return false)
    (else
      (return true))))

(fn IsStatPointsValid
  (if (< (Variables|Default|GetMODStatPoints) (Variables|Default|GetStatPoints))
    (return true)
    (else
      (return false))))

(fn AnyIntegerChanges
  (params (NewParam :type Integer) (NewParam1 :type Integer))
  (if (!= NewParam NewParam1)
    (return true)
    (else
      (return false))))

(fn AnyFloatChanges
  (params (NewParam :type Float%20%28double-precision%29) (NewParam1 :type Float%20%28double-precision%29))
  (if (!= NewParam NewParam1)
    (return true)
    (else
      (return false))))
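; Player shotgun weapon, a child gun Blueprint that takes damage and reload stats from the progression GameInstance and displays its own ammo widget.
; Firing spawns seven bullets from the muzzle socket toward randomized cone traces from the camera.
; Reload adds shells one at a time through delayed loops, which firing breaks, and ammo changes are broadcast through events.
; The gun removes its widget and destroys itself when all ammo is depleted after a shot.
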(event Custom|CheckAmmos
  ;[1 1 1] Destroys Temporary Powerups once Current Ammo and Remaining Ammo are depleted.
  (if (and (<= (Variables|Default|GetCurrent%20Ammo) 0) (<= (Variables|Default|GetRemaining%20Ammo) 0))
    (Widget|RemovefromParent (Variables|Default|GetGun%20Widget))
    (Actor|DestroyActor)))

(event EventBeginPlay
  ;[1 1 1] Setting Defaults; Cannot Set in ConstructionScript(?)
  (bind _asgi_progression_project (Utilities|Casting|CastToGI_ProgressionProject (Game|GetGameInstance)))
  (Utilities|FlowControl|Sequence
    (:then_0
      (Variables|Default|SetDMG (.DMG (Utilities|Struct|BreakS_ShotgunStats (Variables|/Game/Sclopetiator/Blueprints/GI_ProgressionProject.GI_ProgressionProject_C|GetShotgunStats _asgi_progression_project)))))
    (:then_1
      (Variables|Default|SetReload%20Speed (.ReloadSpeed (Utilities|Struct|BreakS_ShotgunStats (Variables|/Game/Sclopetiator/Blueprints/GI_ProgressionProject.GI_ProgressionProject_C|GetShotgunStats _asgi_progression_project)))))))

(event EventReload
  ;[1 1 1] Reload Using Remaining Ammo
  (if (> (Variables|Default|GetRemaining%20Ammo) 0)
    (if (>= (Variables|Default|GetRemaining%20Ammo) (Variables|Default|GetMax%20Ammo))
      ;;[1 1 1] Occurs when Remaining Ammo >= Max Ammo
      (Utilities|ForLoopwithBreakandDelay 1 5 2.0
        (:Loop%20Body
          (bind _output_get (Variables|Default|SetCurrent%20Ammo (+ (Variables|Default|GetCurrent%20Ammo) 1)))
          (Default|CallEonCurrentAmmoModified _output_get)
          (bind _output_get_2 (Variables|Default|SetRemaining%20Ammo (- (Variables|Default|GetRemaining%20Ammo) 1)))
          (Default|CallEonRemainingAmmoModified _output_get_2))
        (:Completed
          (|CallParentFunction)))
      (else
        ;;[1 1 1] Occurs when Remaining Ammo < Max Ammo
        (bind _output_get_3 (Variables|Default|SetRemainingAmmoPlaceholder (Variables|Default|GetRemaining%20Ammo)))
        (Utilities|ForLoopwithBreakandDelay 1 _output_get_3 2.0
          (:Loop%20Body
            (bind _output_get_4 (Variables|Default|SetCurrent%20Ammo (+ (Variables|Default|GetCurrent%20Ammo) 1)))
            (Default|CallEonCurrentAmmoModified _output_get_4)
            (bind _output_get_5 (Variables|Default|SetRemaining%20Ammo (- (Variables|Default|GetRemaining%20Ammo) 1)))
            (Default|CallEonRemainingAmmoModified _output_get_5))
          (:Completed
            (Variables|Default|SetRemainingAmmoPlaceholder (Variables|Default|GetRemaining%20Ammo))
            (|CallParentFunction)))))))

(event EventDecrementCurrentAmmo
  ;[1 1 1] Decrement Current Ammo
  (|CallParentFunction)
  (Default|CallEonCurrentAmmoModified (Variables|Default|GetCurrent%20Ammo)))

(event EventFire
  (bind _skeletalmesh (Variables|Default|GetSkeletalMesh))
  (bind _returnvalue (Transformation|GetSocketLocation _skeletalmesh "ShootSocket"))
  ;[1 1 1] Fires Single Bullet Per Click
  (Utilities|FlowControl|Sequence
    (:then_0
      (bind _asbp_first_person_character (Utilities|Casting|CastToBP_FirstPersonCharacter (Game|GetPlayerCharacter 0)))
      (bind _valid (CallFunction|Checkers (Variables|/Game/FirstPerson/Blueprints/BP_FirstPersonCharacter.BP_FirstPersonCharacter_C|GetisAiming _asbp_first_person_character)))
      (if _valid
        (for _index (range 1 7)
          ;;[1 1 1] Bullet is spawned from the Pistol's ShootSocket, and is aimed at where the player's camera is looking.
          (bind _outhit (Collision|LineTraceByChannel (Transformation|GetWorldLocation (Variables|/Script/Sclopetiator.SclopetiatorCharacter|GetFirstPersonCameraComponent _asbp_first_person_character)) (+ (Transformation|GetWorldLocation (Variables|/Script/Sclopetiator.SclopetiatorCharacter|GetFirstPersonCameraComponent _asbp_first_person_character)) (* (+ (Math|Random|RandomUnitVectorinConeinDegrees (Math|Vector|GetForwardVector (Variables|/Script/Sclopetiator.SclopetiatorCharacter|GetFirstPersonCameraComponent _asbp_first_person_character)) 7.5) (Math|Vector|GetForwardVector (Variables|/Script/Sclopetiator.SclopetiatorCharacter|GetFirstPersonCameraComponent _asbp_first_person_character))) 5e+03)) "TraceTypeQuery1" false 0 "None"))
          (Game|SpawnActorfromClass "/Game/Sclopetiator/Blueprints/BP_Bullet.BP_Bullet_C" (Math|Transform|MakeTransform _returnvalue (Math|Rotator|FindLookatRotation _returnvalue (.TraceEnd (Collision|BreakHitResult _outhit)))) "AlwaysSpawn" "MultiplyWithRoot" 0 (Variables|Default|GetDMG) 0))
        ;;[1 1 1] Decrement Ammo Count
        (CallFunction|DecrementCurrentAmmo)
        (|CallParentFunction)
        (CallFunction|CheckAmmos)))
    (:then_1
      ;[1 1 1] Reload Using Remaining Ammo
      ;;[1 1 1] Occurs when Remaining Ammo >= Max Ammo
      (Utilities|ForLoopwithBreakandDelay 1 5 2.0) ; enters at Break
    )
    (:then_2
      ;;[1 1 1] Occurs when Remaining Ammo < Max Ammo
      (Utilities|ForLoopwithBreakandDelay 1 (stale EventReload _output_get_3) 2.0) ; enters at Break
    )))

(event EventBaseGunSetup
  (bind _returnvalue (Game|GetPlayerController 0))
  ;[1 1 1] On Collision and after Firearm is attached to the Player, set Pistol Widget to Gun Widget and Display to Player.
  (|CallParentFunction)
  (bind _returnvalue_2 (UserInterface|CreateWidget "/Game/Sclopetiator/Blueprints/Widget_Blueprints/WBP_Shotgun.WBP_Shotgun_C" _returnvalue))
  (Variables|Default|SetGun%20Widget _returnvalue_2)
  (bind _asbp_first_person_player_controller (Utilities|Casting|CastToBP_FirstPersonPlayerController _returnvalue))
  (Default|DisplayFirearmWidget _asbp_first_person_player_controller)
  (Default|CallEonCurrentAmmoModified (Variables|Default|GetCurrent%20Ammo))
  (Default|CallEonRemainingAmmoModified (Variables|Default|GetRemaining%20Ammo))
  (Variables|/Script/Engine.RotatingMovementComponent|SetRotationRate (Variables|Default|GetRotatingMovement) "0, 0, 0"))

(event EventTick
  (params (DeltaSeconds :type Float%20%28single-precision%29)))

(fn ConstructionScript
  (|CallParentFunction))
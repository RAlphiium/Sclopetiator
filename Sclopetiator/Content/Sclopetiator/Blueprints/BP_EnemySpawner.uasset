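; BP_EnemySpawner is a spawner actor that creates batches of BP_MeleeEnemy around its Box component.
; SpawnEnemies places the requested number at random reachable nav points, using a radius derived from the box's Y extent.
; It then passes the batch count to BP_WaveChecker and resets it.
; The construction script caches the wave checker reference, while the AssignWaveChecker event called on BeginPlay is empty.
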(event Custom|SpawnEnemies
  (params (TotalEnemiesSpawned :type Integer))
  (bind _box (Variables|Default|GetBox))
  ;[1 1 1] Reusable code to spawn enemies.
  (for _index (range 1 TotalEnemiesSpawned)
    (Game|SpawnActorfromClass "/Game/Sclopetiator/Blueprints/BP_MeleeEnemy.BP_MeleeEnemy_C" (Math|Conversions|ToTransform(Vector) (.RandomLocation (AI|Navigation|GetRandomReachablePointinRadius (Transformation|GetWorldLocation _box) (/ (.y (Variables|/Script/Engine.BoxComponent|GetBoxExtent _box)) 2.0) 0 0))) "AdjustIfPossibleButAlwaysSpawn" "MultiplyWithRoot" 0 0)
    (Variables|Default|SetTotalEnemies (+ (Variables|Default|GetTotalEnemies) 1)))
  (bind _asbp_wave_checker (Utilities|Casting|CastToBP_WaveChecker (Variables|Default|GetWaveChecker)))
  (Default|CalculateTotalEnemies _asbp_wave_checker (Variables|Default|GetTotalEnemies))
  (Variables|Default|SetTotalEnemies 0))

(event Custom|AssignWaveChecker
  ;[1 1 1] Assign WaveChecker
)

(event EventBeginPlay
  ;[1 1 1] Spawns Enemies based on Total Enemies Value
  (CallFunction|AssignWaveChecker))

(fn ConstructionScript
  (bind _outactors (Actor|GetAllActorsOfClass "/Game/Sclopetiator/Blueprints/BP_WaveChecker.BP_WaveChecker_C"))
  (for _array_element _outactors
    (Variables|Default|SetWaveChecker _array_element)))
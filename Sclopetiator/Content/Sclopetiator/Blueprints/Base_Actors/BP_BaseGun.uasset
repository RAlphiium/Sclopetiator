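; BP_BaseGun is the base gun actor, which replaces the player's current gun when the first-person character overlaps its sphere.
; Fire requires aiming, ammo and no cooldown, then spawns damage-carrying projectiles per pellet from the muzzle socket toward randomized cone trace endpoints from the camera.
; Recoil type selects camera shake and sound, a timer handles cooldown, and each shot costs one ammo.
; Reload is only a stub.
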(event OnComponentBeginOverlap(SphereCollision)
  (params (OverlappedComponent :type Primitive%20Component%20Object%20Reference) (OtherActor :type Actor%20Object%20Reference) (OtherComp :type Primitive%20Component%20Object%20Reference) (OtherBodyIndex :type Integer) (bFromSweep :type Boolean) (SweepResult :type Hit%20Result%20Structure%20%28by%20ref%29))
  ;[1 1 1] Writes the Player Character's Current Weapon attribute as this actor's self and runs the First Person Character's AttachWeapon Event.
  (if (== (Utilities|GetClass OtherActor) "/Game/FirstPerson/Blueprints/BP_FirstPersonCharacter.BP_FirstPersonCharacter_C")
    (bind _asbp_first_person_character (Utilities|Casting|CastToBP_FirstPersonCharacter OtherActor))
    (Variables|Default|SetAs%20BP%20First%20Person%20Character _asbp_first_person_character)
    (Variables|/Script/Engine.PrimitiveComponent|SetbGenerateOverlapEvents (Variables|Default|GetSphereCollision) false)
    (CallFunction|BaseGunSetup)))

(event Custom|BaseGun%20Setup
  (bind _as_bp_first_person_character (Variables|Default|GetAs%20BP%20First%20Person%20Character))
  ;[1 1 1] Writes the Player Character's Current Weapon attribute as this actor's self and runs the First Person Character's AttachWeapon Event.
  (bind _currentgun (Variables|/Game/FirstPerson/Blueprints/BP_FirstPersonCharacter.BP_FirstPersonCharacter_C|GetCurrentGun _as_bp_first_person_character)
    (:then
      (Widget|RemovefromParent (Variables|BP_BaseGun_C|GetGun%20Widget _currentgun))
      (Transformation|DetachFromActor _currentgun "KeepRelative" "KeepRelative" "KeepRelative")
      (Actor|DestroyActor _currentgun)
      (Variables|/Game/FirstPerson/Blueprints/BP_FirstPersonCharacter.BP_FirstPersonCharacter_C|SetCurrentGun _as_bp_first_person_character self)
      (Default|AttachGun _as_bp_first_person_character))
    (:else
      (Variables|/Game/FirstPerson/Blueprints/BP_FirstPersonCharacter.BP_FirstPersonCharacter_C|SetCurrentGun _as_bp_first_person_character self)
      (Default|AttachGun _as_bp_first_person_character))))

(event Custom|Fire
  (bind _returnvalue (Transformation|GetActorLocation))
  (bind _skeletalmesh (Variables|Default|GetSkeletalMesh))
  (bind _as_bp_first_person_character (Variables|Default|GetAs%20BP%20First%20Person%20Character))
  (bind _returnvalue_2 (Transformation|GetActorLocation _as_bp_first_person_character))
  (bind _returnvalue_3 (Transformation|GetSocketLocation _skeletalmesh "ShootSocket"))
  ;[1 1 1] Event that Derived Actors can access. Will need to enable Gun Actors to shoot.
  (bind _asbp_first_person_character (Utilities|Casting|CastToBP_FirstPersonCharacter (Game|GetPlayerCharacter 0)))
  (bind _valid (CallFunction|Checkers (Variables|/Game/FirstPerson/Blueprints/BP_FirstPersonCharacter.BP_FirstPersonCharacter_C|GetisAiming _asbp_first_person_character)))
  (if _valid
    (if (Variables|Default|GetisNotOnCooldown)
      (Variables|Default|SetisNotOnCooldown false)
      (for _index (range 1 (Variables|Default|GetNumberOfPellets))
        ;;[1 1 1] Bullet is spawned from the Pistol's ShootSocket, and is aimed at where the player's camera is looking.
        (bind _outhit (Collision|LineTraceByChannel (Transformation|GetWorldLocation (Variables|/Script/Sclopetiator.SclopetiatorCharacter|GetFirstPersonCameraComponent _asbp_first_person_character)) (+ (Transformation|GetWorldLocation (Variables|/Script/Sclopetiator.SclopetiatorCharacter|GetFirstPersonCameraComponent _asbp_first_person_character)) (* (Math|Random|RandomUnitVectorinConeinDegrees (Math|Vector|GetForwardVector (Variables|/Script/Sclopetiator.SclopetiatorCharacter|GetFirstPersonCameraComponent _asbp_first_person_character)) (Variables|Default|GetOffset)) 5e+03)) "TraceTypeQuery1" false 0 "None"))
        (Game|SpawnActorfromClass "/Game/Sclopetiator/Blueprints/BP_PlayerProjectile.BP_PlayerProjectile_C" (Math|Transform|MakeTransform _returnvalue_3 (Math|Rotator|FindLookatRotation _returnvalue_3 (.TraceEnd (Collision|BreakHitResult _outhit)))) "AlwaysSpawn" "MultiplyWithRoot" 0 (Variables|Default|GetDMG) 0)
        (Utilities|Time|SetTimerbyEvent (EventDispatchers|CreateEvent :!event Custom|ResetFireCooldown) (Variables|Default|GetFireCooldownTime))
        (switch Utilities|FlowControl|Switch|SwitchonE_RecoilType (Variables|Default|GetRecoilType)
          (:NewEnumerator1
            (Camera|PlayWorldCameraShake "/Game/Sclopetiator/Blueprints/BP_PistolCameraShake.BP_PistolCameraShake_C" _returnvalue_2 0.0 1e+02)
            (Audio|PlaySoundatLocation "/Game/Sclopetiator/Assets/Audio/MetaSound/MS_PistolFire.MS_PistolFire" _returnvalue "0, 0, 0" 1.0 1.0 0.0 0 0 0 0))
          (:NewEnumerator2
            (Camera|PlayWorldCameraShake "/Game/Sclopetiator/Blueprints/BP_ShotgunCameraShake.BP_ShotgunCameraShake_C" _returnvalue_2 0.0 1e+02)
            (Audio|PlaySoundatLocation "/Game/Sclopetiator/Assets/Audio/MetaSound/MS_ShotgunFire.MS_ShotgunFire" _returnvalue "0, 0, 0" 1.0 1.0 0.0 0 0 0 0))
          (:NewEnumerator3
            (Camera|PlayWorldCameraShake "/Game/Sclopetiator/Blueprints/BP_RifleCameraShake.BP_RifleCameraShake_C" _returnvalue_2 0.0 1e+02)
            (Audio|PlaySoundatLocation "/Game/Sclopetiator/Assets/Audio/MetaSound/MS_RifleFire.MS_RifleFire" _returnvalue "0, 0, 0" 1.0 1.0 0.0 0 0 0 0))))
      ;;[1 1 1] Decrement Ammo Count
      (CallFunction|DecrementCurrentAmmo))))

(event Custom|Reload
  ;[1 1 1] Event that Derived Actors can access. Will need to enable Gun Actors to shoot.
  (if (< (Variables|Default|GetCurrent%20Ammo) (Variables|Default|GetMax%20Ammo))
    _))

(event Custom|DecrementCurrentAmmo
  ;[1 1 1] Event that Derived Actors can access. Decrements Firearm's Current Ammo Count by 1.
  (Variables|Default|SetCurrent%20Ammo (- (Variables|Default|GetCurrent%20Ammo) 1)))

(event Custom|ResetFireCooldown
  ;[1 1 1] Reset FireCooldown
  (Variables|Default|SetisNotOnCooldown true))

(event Custom|ResetReloadCooldown
  ;[1 1 1] Reset FireCooldown
  (Variables|Default|SetisNotReloading true))

(event Custom|EquipDefaultFirearm
  ;[1 1 1] Spawn Pistol on Player Transform
  (Game|SpawnActorfromClass "/Game/Sclopetiator/Blueprints/BP_Pistol.BP_Pistol_C" (Transformation|GetActorTransform (Variables|Default|GetAs%20BP%20First%20Person%20Character)) "Undefined" "MultiplyWithRoot" 0 0))

(fn ConstructionScript)

(fn Checkers
  (params (isAiming :type Boolean))
  ;[1 1 1] Checks if there is still ammo in Firearm
  (if (== isAiming true)
    (if (> (Variables|Default|GetCurrent%20Ammo) 0)
      (return true)
      (else
        _)))
  (return false))
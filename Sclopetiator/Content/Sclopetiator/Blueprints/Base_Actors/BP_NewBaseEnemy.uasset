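; BP_NewBaseEnemy is a base enemy character with health, movement speed and a weapon.
; On BeginPlay it applies its walk speed and caches the level's BP_WaveChecker.
; When DecrementHealth empties its health, it decrements the wave's enemy count, rolls against player Luck to spawn BP_RandomItemDrop, then destroys its weapon and itself.
; AttackEvent is an empty stub, a lunge sits unconnected, and Tick prints health for debugging.
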(event Custom|AttackEvent
  ;[1 1 1] Attack Event
)

(event Custom|AssignWaveChecker
  ;[1 1 1] Assign WaveChecker
  (bind _outactors (Actor|GetAllActorsOfClass "/Game/Sclopetiator/Blueprints/BP_WaveChecker.BP_WaveChecker_C"))
  (for _array_element _outactors
    (Variables|Default|SetWaveChecker _array_element)))

(event Custom|SetSpeed
  ;[1 1 1] Set Default Speed
  (Variables|/Script/Engine.CharacterMovementComponent|SetMaxWalkSpeed (Variables|Character|GetCharacterMovement) (Variables|Default|GetSpeed)))

(event Custom|DecrementHealth
  (params (DMG :type Integer))
  ;[1 1 1] Deducts HP using DMG Value. If HP <=0, Call Event Dispatcher and destroy self.
  (bind _output_get (Variables|Default|SetHealth (- (Variables|Default|GetHealth) DMG)))
  (if (<= _output_get 0)
    (Default|DecrementTotalEnemies (Variables|Default|GetWaveChecker))
    (CallFunction|AbilitytoDropItem)
    (Actor|DestroyActor (Variables|Default|GetWeapon))
    (Actor|DestroyActor)))

(event Custom|AbilityToDropItem
  ;[1 1 1] Calculates whether an Item will be dropped depending on Player Luck and spawns RandomItemDrop Actor
  (bind _asbp_first_person_character (Utilities|Casting|CastToBP_FirstPersonCharacter (Game|GetPlayerCharacter 0)))
  (bind _output_get (Variables|Default|SetRandomFloat (Math|Random|RandomFloatinRange 0.0 1e+02)))
  (if (<= _output_get (Variables|/Script/Sclopetiator.SclopetiatorCharacter|GetLuck _asbp_first_person_character))
    (Game|SpawnActorfromClass "/Game/Sclopetiator/Blueprints/BP_RandomItemDrop.BP_RandomItemDrop_C" (Transformation|GetActorTransform) "AlwaysSpawn" "MultiplyWithRoot" 0 0)))

(event Custom|SetDefaults
  ;[1 1 1] Set Defaults
  (CallFunction|SetSpeed))

(event EventTick
  (params (DeltaSeconds :type Float%20%28single-precision%29))
  (Development|PrintString (Utilities|String|ToString(Integer) (Variables|Default|GetHealth)) true true "(R=0.000000,G=0.660000,B=1.000000,A=1.000000)" (Utilities|Time|GetWorldDeltaSeconds)))

(event EventBeginPlay
  ;[1 1 1] Set Default Variables
  (CallFunction|SetDefaults)
  (CallFunction|AssignWaveChecker))

(fn ConstructionScript)
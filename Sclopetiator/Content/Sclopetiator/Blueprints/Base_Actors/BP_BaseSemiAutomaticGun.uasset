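; BP_BaseSemiAutomaticGun is the base gun Blueprint for semi-automatic weapons such as the pistol and shotgun.
; It extends the parent's BaseGunSetup to switch the first player controller's Enhanced Input contexts.
; The switch adds IMC_SemiAutomaticFire and removes IMC_AutomaticFire.
; Its Fire override only calls the parent, so this class itself adds no firing logic.
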(event Custom|ModifyPlayerInputMappings
  ;[1 1 1] Adds new Input Mapping for Semi-Automatic Guns, such as Pistol and Shotgun.
  (bind _asplayer_controller (Utilities|Casting|CastToPlayerController (Game|GetPlayerController 0)))
  (Utilities|IsValid (PlayerController|LocalPlayerSubsystems|GetEnhancedInputLocalPlayerSubsystem _asplayer_controller)
    (:Is%20Valid
      (Input|AddMappingContext (PlayerController|LocalPlayerSubsystems|GetEnhancedInputLocalPlayerSubsystem _asplayer_controller) "/Game/Sclopetiator/Inputs/IMC_SemiAutomaticFire.IMC_SemiAutomaticFire" 1 "(bIgnoreAllPressedKeysUntilRelease=True,bForceImmediately=False,bNotifyUserSettings=False)")
      (Input|RemoveMappingContext (PlayerController|LocalPlayerSubsystems|GetEnhancedInputLocalPlayerSubsystem _asplayer_controller) "/Game/Sclopetiator/Inputs/IMC_AutomaticFire.IMC_AutomaticFire" "(bIgnoreAllPressedKeysUntilRelease=True,bForceImmediately=False,bNotifyUserSettings=False)"))))

(event EventBeginPlay
  (|CallParentFunction) ; This node is disabled and will not be called.\nDrag off pins to build functionality.
)

(event Collision|EventActorBeginOverlap
  (params (OtherActor :type Actor%20Object%20Reference))
  (|CallParentFunction OtherActor) ; This node is disabled and will not be called.\nDrag off pins to build functionality.
)

(event EventTick
  (params (DeltaSeconds :type Float%20%28single-precision%29))
  (|CallParentFunction DeltaSeconds) ; This node is disabled and will not be called.\nDrag off pins to build functionality.
)

(event EventBaseGunSetup
  ;[1 1 1] Overrides Parent function.
  (|CallParentFunction)
  (CallFunction|ModifyPlayerInputMappings))

(event EventFire
  ;[1 1 1] Overrides Parent Function
  (|CallParentFunction))

(fn ConstructionScript
  (|CallParentFunction))
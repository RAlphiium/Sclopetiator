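; Base enemy that roams randomly, chases the player on sight and reports its death to the wave checker.
; On BeginPlay it applies its speed, caches BP_WaveChecker, starts looping AI roam moves and binds a health-modified dispatcher.
; PawnSensing triggers a chase of BP_FirstPersonCharacter, with a retriggerable delay returning it to roaming after sightings stop.
; The dispatcher handler subtracts damage, then at zero health decrements the wave's enemy count and destroys the actor.
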(event OnSeePawn(PawnSensing)
  (params (Pawn :type Pawn%20Object%20Reference))
  ;[1 1 1] Enemy - Player Detection
  (if (== (Utilities|GetClass Pawn) "/Game/FirstPerson/Blueprints/BP_FirstPersonCharacter.BP_FirstPersonCharacter_C")
    (Variables|Default|SetPlayerTarget Pawn)
    (Utilities|FlowControl|Sequence
      (:then_0
        (AI|AIMoveTo self "0, 0, 0" (Variables|Default|GetPlayerTarget) 5.0 false))
      (:then_1
        (Utilities|FlowControl|RetriggerableDelay 3.0)
        (CallFunction|RandomRoam)))))

(event Custom|Eon_HealthModified_Event
  (params (DMG :type Integer))
  ;[1 1 1] Deducts HP using DMG Value. If HP <=0, Call Event Dispatcher and destroy self.
  (bind _output_get (Variables|Default|SetHealth (- (Variables|Default|GetHealth) DMG)))
  (if (<= _output_get 0)
    (bind _asbp_wave_checker (Utilities|Casting|CastToBP_WaveChecker (Variables|Default|GetWaveChecker)))
    (Default|DecrementTotalEnemies _asbp_wave_checker)
    (Actor|DestroyActor)))

(event Custom|AssignWaveChecker
  ;[1 1 1] Assign WaveChecker
  (bind _outactors (Actor|GetAllActorsOfClass "/Game/Sclopetiator/Blueprints/BP_WaveChecker.BP_WaveChecker_C"))
  (for _array_element _outactors
    (Variables|Default|SetWaveChecker _array_element)))

(event Custom|SetSpeed
  ;[1 1 1] Set Speed
  (Variables|/Script/Engine.CharacterMovementComponent|SetMaxWalkSpeed (Variables|Character|GetCharacterMovement self) (Variables|Default|GetSpeed)))

(event Custom|RandomRoam
  (bind _self self)
  ;[1 1 1] Enemy - Random Roaming
  (AI|AIMoveTo _self (.RandomLocation (AI|Navigation|GetRandomReachablePointinRadius (Transformation|GetActorLocation _self) (Variables|Default|GetRoamingRadius) 0 0)) 0 5.0 false
    (:OnSuccess
      (CallFunction|RandomRoam))))

(event EventBeginPlay
  ;[1 1 1] Enemy will roam immediately after spawning.
  (CallFunction|SetSpeed)
  (CallFunction|AssignWaveChecker)
  (CallFunction|RandomRoam)
  ;;[1 1 1] Binds Event - DMG Taken
  (EventDispatchers|BindEventtoEonHealthModified (EventDispatchers|CreateEvent :!event Custom|Eon_HealthModified_Event)))

(event EventTick
  (params (DeltaSeconds :type Float%20%28single-precision%29))
  ;[1 1 1] Debugger to check enemy hp
)

(fn ConstructionScript)
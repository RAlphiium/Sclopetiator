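; BP_BaseAutomaticGun is a base gun Blueprint for automatic weapons such as rifles, extending a parent base gun.
; On gun setup it runs the parent setup, then swaps the first player's Enhanced Input contexts, adding IMC_AutomaticFire and removing IMC_SemiAutomaticFire.
; Fire and the construction script only call their parent versions, so the input mapping swap is its only added behavior.
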(event Custom|ModifyPlayerInputMappings
  ;[1 1 1] Adds new Input Mapping for Automatic Guns, such as Rifle.
  (bind _asplayer_controller (Utilities|Casting|CastToPlayerController (Game|GetPlayerController 0)))
  (Utilities|IsValid (PlayerController|LocalPlayerSubsystems|GetEnhancedInputLocalPlayerSubsystem _asplayer_controller)
    (:Is%20Valid
      (Input|AddMappingContext (PlayerController|LocalPlayerSubsystems|GetEnhancedInputLocalPlayerSubsystem _asplayer_controller) "/Game/Sclopetiator/Inputs/IMC_AutomaticFire.IMC_AutomaticFire" 1 "(bIgnoreAllPressedKeysUntilRelease=True,bForceImmediately=False,bNotifyUserSettings=False)")
      (Input|RemoveMappingContext (PlayerController|LocalPlayerSubsystems|GetEnhancedInputLocalPlayerSubsystem _asplayer_controller) "/Game/Sclopetiator/Inputs/IMC_SemiAutomaticFire.IMC_SemiAutomaticFire" "(bIgnoreAllPressedKeysUntilRelease=True,bForceImmediately=False,bNotifyUserSettings=False)"))))

(event EventBeginPlay)

(event Collision|EventActorBeginOverlap
  (params (OtherActor :type Actor%20Object%20Reference)))

(event EventTick
  (params (DeltaSeconds :type Float%20%28single-precision%29)))

(event EventBaseGunSetup
  ;[1 1 1] Overrides Parent function.
  (|CallParentFunction)
  (CallFunction|ModifyPlayerInputMappings))

(event EventFire
  ;[1 1 1] Overrides Parent Function
  (|CallParentFunction))

(fn ConstructionScript
  (|CallParentFunction))
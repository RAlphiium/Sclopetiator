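; Melee enemy Blueprint that spawns with a sword and performs a lunging slash attack.
; On BeginPlay it spawns a BP_Sword, stores it as its weapon and attaches the sword's mesh to the hand socket before calling the parent.
; Its attack launches the character forward horizontally, calls the parent attack and plays a slash montage.
; The sword's box generates overlap events from montage start until completion, limiting the hit window to the swing.
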(event EventBeginPlay
  ;[1 1 1] Attaches Sword to Melee Enemy
  (bind _returnvalue (Game|SpawnActorfromClass "/Game/Sclopetiator/Blueprints/BP_Sword.BP_Sword_C" (Transformation|GetActorTransform) "Undefined" "MultiplyWithRoot" 0 0))
  (bind _output_get (Variables|Default|SetWeapon _returnvalue))
  (Transformation|AttachComponentToComponent (Variables|/Game/Sclopetiator/Blueprints/Base_Actors/BP_BaseEnemyWeapon.BP_BaseEnemyWeapon_C|GetSkeletalMesh _output_get) (Variables|Character|GetMesh) "SwordSocket" "KeepRelative" "KeepRelative" "KeepRelative" true)
  (|CallParentFunction))

(event EventAttackEvent
  (bind _weapon (Variables|Default|GetWeapon))
  (bind _box (Variables|/Game/Sclopetiator/Blueprints/Base_Actors/BP_BaseEnemyWeapon.BP_BaseEnemyWeapon_C|GetBox _weapon))
  ;[1 1 1] Melee Attack; Launch Character
  (Character|LaunchCharacter (+ (* (Transformation|GetActorForwardVector) "1.000000,1.000000,0.000000" 1.5e+03) "0.000000,0.000000,50.000000") false false)
  (|CallParentFunction)
  (Animation|Montage|PlayMontage (Variables|Character|GetMesh) "/Game/Sclopetiator/Assets/EnemyCharacters/MeleeEnemy/Animations/Montages/Montage_Stable_Sword_Outward_Slash.Montage_Stable_Sword_Outward_Slash" 1.25
    (:then
      (Variables|/Script/Engine.PrimitiveComponent|SetbGenerateOverlapEvents _box true))
    (:OnCompleted
      (Variables|/Script/Engine.PrimitiveComponent|SetbGenerateOverlapEvents _box false))))

(fn ConstructionScript
  (|CallParentFunction))
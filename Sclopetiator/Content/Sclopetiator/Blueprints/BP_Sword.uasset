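; BP_Sword is a melee hazard actor that damages and knocks back the first-person player when its Box collision overlaps them.
; On overlap it turns off the Box's overlap events, so it hits once until they are re-enabled outside this Blueprint.
; HarmPlayer launches the player opposite their own facing with a slight lift, plays a detection sound at the sword and calls HealthModified on the character.
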(event OnComponentBeginOverlap(Box)
  (params (OverlappedComponent :type Primitive%20Component%20Object%20Reference) (OtherActor :type Actor%20Object%20Reference) (OtherComp :type Primitive%20Component%20Object%20Reference) (OtherBodyIndex :type Integer) (bFromSweep :type Boolean) (SweepResult :type Hit%20Result%20Structure%20%28by%20ref%29))
  (bind _box (Variables|Default|GetBox))
  ;[1 1 1] On Success, Damage and Knockback Player
  (if (== (Utilities|GetClass OtherActor) "/Game/FirstPerson/Blueprints/BP_FirstPersonCharacter.BP_FirstPersonCharacter_C")
    (if (Variables|/Script/Engine.PrimitiveComponent|GetbGenerateOverlapEvents _box)
      (Utilities|FlowControl|Sequence
        (:then_0
          (Variables|/Script/Engine.PrimitiveComponent|SetbGenerateOverlapEvents _box false))
        (:then_1
          (CallFunction|HarmPlayer))))))

(event Custom|HarmPlayer
  (bind _returnvalue (Game|GetPlayerCharacter 0))
  ;[1 1 1] Apply Impulse and Damage
  (bind _asbp_first_person_character (Utilities|Casting|CastToBP_FirstPersonCharacter _returnvalue))
  (Utilities|FlowControl|Sequence
    (:then_0
      (Physics|AddImpulse (Variables|/Script/Engine.Character|GetCharacterMovement _asbp_first_person_character) (* (+ (* (Math|Vector|GetForwardVector (Variables|/Script/Engine.Character|GetCapsuleComponent _returnvalue)) -1.0) "0.000000,0.000000,0.500000") 6e+02) true)
      (Audio|PlaySoundatLocation "/Game/Sclopetiator/Assets/Audio/MetaSound/MS_SwordDetect.MS_SwordDetect" (Transformation|GetActorLocation) "0, 0, 0" 1.0 1.0 0.0 0 0 0 0))
    (:then_1
      (Class|SclopetiatorCharacter|HealthModified _asbp_first_person_character 1))))

(fn ConstructionScript
  (|CallParentFunction))
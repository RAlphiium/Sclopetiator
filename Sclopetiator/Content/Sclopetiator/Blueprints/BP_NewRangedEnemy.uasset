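; Ranged enemy Blueprint that attacks the player with a bow, extending a parent enemy's BeginPlay and attack events.
; On BeginPlay it spawns a bow, stores it as its weapon and attaches it to the mesh's bow socket.
; Attacks play a slowed aim montage and sound, wait out a focus delay, then play recoil and release sound.
; FireArrow spawns a projectile at the arrow socket, rotated toward the player and carrying the enemy's damage value.
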(event Custom|FireArrow
  (bind _mesh (Variables|Character|GetMesh))
  (bind _returnvalue (Transformation|GetSocketLocation _mesh "ArrowSocket"))
  ;[1 1 1] Spawn Arrow and Fire towards Player
  (bind _asbp_first_person_character (Utilities|Casting|CastToBP_FirstPersonCharacter (Game|GetPlayerCharacter 0)))
  (Game|SpawnActorfromClass "/Game/Sclopetiator/Blueprints/BP_EnemyProjectile.BP_EnemyProjectile_C" (Math|Transform|MakeTransform _returnvalue (Math|Rotator|FindLookatRotation _returnvalue (Transformation|GetActorLocation _asbp_first_person_character)) "1.000000,1.000000,1.000000") "Undefined" "MultiplyWithRoot" 0 (Variables|Default|GetDMG) 0))

(event EventBeginPlay
  ;[1 1 1] Attaches Bow to Ranged Enemy
  (bind _returnvalue (Game|SpawnActorfromClass "/Game/Sclopetiator/Blueprints/BP_Bow.BP_Bow_C" (Transformation|GetActorTransform) "Undefined" "MultiplyWithRoot" 0 0))
  (bind _output_get (Variables|Default|SetWeapon _returnvalue))
  (Transformation|AttachComponentToComponent (Variables|/Game/Sclopetiator/Blueprints/Base_Actors/BP_BaseEnemyWeapon.BP_BaseEnemyWeapon_C|GetSkeletalMesh _output_get) (Variables|Character|GetMesh) "BowSocket" "KeepRelative" "KeepRelative" "KeepRelative" true)
  (|CallParentFunction))

(event EventAttackEvent
  (bind _returnvalue (Transformation|GetActorLocation))
  ;[1 1 1] Ranged Attack
  (Animation|PlayAnimMontage "/Game/Sclopetiator/Assets/EnemyCharacters/RangedEnemy/Animations/Montages/Montage_Standing_Aim_Idle_01.Montage_Standing_Aim_Idle_01" 0.2 "None")
  (Audio|PlaySoundatLocation "/Game/Sclopetiator/Assets/Audio/MetaSound/MS_BowAim.MS_BowAim" _returnvalue "0, 0, 0" 1.0 1.0 0.0 0 0 0 0)
  (Utilities|FlowControl|Delay (Variables|Default|GetFocusTime))
  (Animation|PlayAnimMontage "/Game/Sclopetiator/Assets/EnemyCharacters/RangedEnemy/Animations/Montages/Montage_Standing_Aim_Recoil.Montage_Standing_Aim_Recoil" 1.0 "None")
  (Audio|PlaySoundatLocation "/Game/Sclopetiator/Assets/Audio/MetaSound/MS_BowRelease.MS_BowRelease" _returnvalue "0, 0, 0" 1.0 1.0 0.0 0 0 0 0)
  (CallFunction|FireArrow)
  (|CallParentFunction))

(fn ConstructionScript
  (|CallParentFunction))
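; BP_Bullet is a projectile that damages enemies and awards the player score on hit.
; Its Box overlap accepts only exact BP_BaseEnemy or BP_MeleeEnemy classes, then destroys the bullet to prevent piercing.
; It tests the enemy's Head before its Body, applying the same DMG to either while awarding more points for headshots through BP_FirstPersonCharacter.
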(event OnComponentBeginOverlap(Box)
  (params (OverlappedComponent :type Primitive%20Component%20Object%20Reference) (OtherActor :type Actor%20Object%20Reference) (OtherComp :type Primitive%20Component%20Object%20Reference) (OtherBodyIndex :type Integer) (bFromSweep :type Boolean) (SweepResult :type Hit%20Result%20Structure%20%28by%20ref%29))
  (bind _returnvalue (Utilities|GetClass OtherActor))
  ;[1 1 1] Bullet Collision
  (if (or (== _returnvalue "/Game/Sclopetiator/Blueprints/Base_Actors/BP_BaseEnemy.BP_BaseEnemy_C") (== _returnvalue "/Game/Sclopetiator/Blueprints/BP_MeleeEnemy.BP_MeleeEnemy_C"))
    (bind _asbp_base_enemy (Utilities|Casting|CastToBP_BaseEnemy OtherActor))
    (CallFunction|CheckHead _asbp_base_enemy)
    ;;[1 1 1] Prevents Piercing Effect
    (Actor|DestroyActor)))

(event Custom|CheckHead
  (params (Enemy :type BP%20Base%20Enemy%20Object%20Reference))
  ;[1 1 1] Checks if Head Component of Enemy has been Overlapped.
  (if (Collision|IsOverlappingActor (Variables|/Game/Sclopetiator/Blueprints/Base_Actors/BP_BaseEnemy.BP_BaseEnemy_C|GetHead Enemy) self :!class /Script/Engine.PrimitiveComponent)
    (Default|EonHealthModifiedEvent Enemy (Variables|Default|GetDMG))
    (bind _asbp_first_person_character (Utilities|Casting|CastToBP_FirstPersonCharacter (Game|GetPlayerCharacter 0)))
    (Class|SclopetiatorCharacter|ScorePointsModified _asbp_first_person_character 100)
    (else
      (CallFunction|CheckBody Enemy))))

(event Custom|CheckBody
  (params (Enemy :type BP%20Base%20Enemy%20Object%20Reference))
  ;[1 1 1] Checks if Body Component of Enemy has been Overlapped.
  (if (Collision|IsOverlappingActor (Variables|/Game/Sclopetiator/Blueprints/Base_Actors/BP_BaseEnemy.BP_BaseEnemy_C|GetBody Enemy) self :!class /Script/Engine.PrimitiveComponent)
    (Default|EonHealthModifiedEvent Enemy (Variables|Default|GetDMG))
    (bind _asbp_first_person_character (Utilities|Casting|CastToBP_FirstPersonCharacter (Game|GetPlayerCharacter 0)))
    (Class|SclopetiatorCharacter|ScorePointsModified _asbp_first_person_character 50)))

(fn ConstructionScript)
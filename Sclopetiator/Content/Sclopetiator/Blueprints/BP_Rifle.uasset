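; Rifle firearm Blueprint, extending a base gun, that acts as a temporary powerup and destroys itself once all ammo is spent.
; BeginPlay pulls damage and reload speed from the GameInstance and sets the fire cooldown.
; Setup creates the rifle HUD widget, while firing and reloading push ammo changes through modified-ammo events.
; Reload moves reserve ammo into the magazine immediately, then starts a reload timer; Tick prints debug state.
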(event Custom|CheckAmmos
  ;[1 1 1] Destroys Temporary Powerups once Current Ammo and Remaining Ammo are depleted.
  (if (and (<= (Variables|Default|GetCurrent%20Ammo) 0) (<= (Variables|Default|GetRemaining%20Ammo) 0))
    (Widget|RemovefromParent (Variables|Default|GetGun%20Widget))
    (Actor|DestroyActor)))

(event Custom|AllocateRemainingToCurrent
  (params (Remaining>Max? :type Boolean))
  ;[1 1 1] Outcome 1: If Remaining > Max, Outcome 2: If Remaining > Max & Current + Remaining < max, Outcome 3: If Remaining > Max & Current + Remaining > Max
  (if Remaining>Max?
    (bind _output_get (Variables|Default|SetRequiredAmmo (- (Variables|Default|GetMax%20Ammo) (Variables|Default|GetCurrent%20Ammo))))
    (Variables|Default|SetCurrent%20Ammo (+ (Variables|Default|GetCurrent%20Ammo) _output_get))
    (Variables|Default|SetRemaining%20Ammo (- (Variables|Default|GetRemaining%20Ammo) _output_get))
    (Development|PrintString "Outcome: 1")
    (elif (< (Variables|Default|GetMax%20Ammo) (+ (Variables|Default|GetCurrent%20Ammo) (Variables|Default|GetRemaining%20Ammo)))
      (bind _output_get_2 (Variables|Default|SetRequiredAmmo (- (Variables|Default|GetMax%20Ammo) (Variables|Default|GetCurrent%20Ammo))))
      (Variables|Default|SetCurrent%20Ammo (+ (Variables|Default|GetCurrent%20Ammo) _output_get_2))
      (Variables|Default|SetRemaining%20Ammo (- (Variables|Default|GetRemaining%20Ammo) _output_get_2))
      (Development|PrintString "Outcome: 2")
      (else
        (Variables|Default|SetCurrent%20Ammo (+ (Variables|Default|GetCurrent%20Ammo) (Variables|Default|GetRemaining%20Ammo)))
        (Variables|Default|SetRemaining%20Ammo (- (Variables|Default|GetRemaining%20Ammo) (Variables|Default|GetRemaining%20Ammo)))
        (Development|PrintString "Outcome: 3")))))

(event EventBaseGunSetup
  (bind _returnvalue (Game|GetPlayerController 0))
  ;[1 1 1] On Collision and after Firearm is attached to the Player, set Pistol Widget to Gun Widget and Display to Player.
  (|CallParentFunction)
  (bind _returnvalue_2 (UserInterface|CreateWidget "/Game/Sclopetiator/Blueprints/Widget_Blueprints/WBP_Rifle.WBP_Rifle_C" _returnvalue))
  (Variables|Default|SetGun%20Widget _returnvalue_2)
  (bind _asbp_first_person_player_controller (Utilities|Casting|CastToBP_FirstPersonPlayerController _returnvalue))
  (Default|DisplayFirearmWidget _asbp_first_person_player_controller)
  (Default|CallEonCurrentAmmoModified (Variables|Default|GetCurrent%20Ammo))
  (Default|CallEonRemainingAmmoModified (Variables|Default|GetRemaining%20Ammo))
  (Variables|/Script/Engine.RotatingMovementComponent|SetRotationRate (Variables|Default|GetRotatingMovement) "0, 0, 0"))

(event EventDecrementCurrentAmmo
  ;[1 1 1] Decrement Current Ammo
  (|CallParentFunction)
  (Default|CallEonCurrentAmmoModified (Variables|Default|GetCurrent%20Ammo)))

(event EventFire
  ;[1 1 1] Fires Bullet Per Click
  (|CallParentFunction)
  (CallFunction|CheckAmmos))

(event EventReload
  (bind _remaining_ammo (Variables|Default|GetRemaining%20Ammo))
  ;[1 1 1] Reload
  (if (Variables|Default|GetisNotReloading)
    (Variables|Default|SetisNotReloading false)
    (if (> _remaining_ammo 0)
      (CallFunction|AllocateRemainingtoCurrent (>= _remaining_ammo (Variables|Default|GetMax%20Ammo)))
      (Utilities|Time|SetTimerbyEvent (EventDispatchers|CreateEvent :!event ResetReloadCooldown) (Variables|Default|GetReload%20Speed))
      (Default|CallEonCurrentAmmoModified (Variables|Default|GetCurrent%20Ammo))
      (Default|CallEonRemainingAmmoModified (Variables|Default|GetRemaining%20Ammo)))))

(event EventTick
  (params (DeltaSeconds :type Float%20%28single-precision%29))
  (bind _asbp_first_person_character (Utilities|Casting|CastToBP_FirstPersonCharacter (Game|GetPlayerCharacter 0)))
  (Development|PrintString (Utilities|String|ToString(Text) (Utilities|Text|FormatText "IsNotReloading: {x} 
IsNotCooldown: {a} 
IsAiming: {y} 
Ammo: {z}" (Variables|Default|GetisNotReloading) (Variables|/Script/Sclopetiator.SclopetiatorCharacter|GetisAiming _asbp_first_person_character) (Variables|Default|GetCurrent%20Ammo) (Variables|Default|GetisNotOnCooldown))) true true "(R=0.000000,G=0.660000,B=1.000000,A=1.000000)" (Utilities|Time|GetWorldDeltaSeconds)))

(event EventBeginPlay
  ;[1 1 1] Setting Defaults; Cannot Set in ConstructionScript(?)
  (bind _asgi_sclopetiator (Utilities|Casting|CastToGI_Sclopetiator (Game|GetGameInstance)))
  (Utilities|FlowControl|Sequence
    (:then_0
      (Variables|Default|SetDMG (.DMG (Utilities|Struct|BreakFirearmStats (Variables|/Script/Sclopetiator.VS_SclopetiatorGI|GetRifleStats _asgi_sclopetiator)))))
    (:then_1
      (Variables|Default|SetReload%20Speed (.ReloadSpeed (Utilities|Struct|BreakFirearmStats (Variables|/Script/Sclopetiator.VS_SclopetiatorGI|GetRifleStats _asgi_sclopetiator)))))
    (:then_2
      (Variables|Default|SetFireCooldownTime 0.1))))

(fn ConstructionScript
  (|CallParentFunction))
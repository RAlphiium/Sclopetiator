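; BP_Pistol is the pistol firearm, a child of a base gun that supplies single-shot firing.
; BeginPlay loads damage and reload speed from the game instance's pistol stats and sets the fire cooldown.
; Gun setup creates the pistol widget, displays it through the player controller and stops the rotating movement.
; Reload refills ammo immediately, blocks firing and starts reload-length timers, while ammo changes are broadcast through an event.
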(event EventDecrementCurrentAmmo
  ;[1 1 1] Decrement Current Ammo
  (|CallParentFunction)
  (Default|CallEonCurrentAmmoModified (Variables|Default|GetCurrent%20Ammo)))

(event EventBeginPlay
  ;[1 1 1] Setting Defaults; Cannot Set in ConstructionScript(?)
  (bind _asgi_sclopetiator (Utilities|Casting|CastToGI_Sclopetiator (Game|GetGameInstance)))
  (Utilities|FlowControl|Sequence
    (:then_0
      (Variables|Default|SetDMG (.DMG (Utilities|Struct|BreakFirearmStats (Variables|/Script/Sclopetiator.VS_SclopetiatorGI|GetPistolStats _asgi_sclopetiator)))))
    (:then_1
      (Variables|Default|SetReload%20Speed (.ReloadSpeed (Utilities|Struct|BreakFirearmStats (Variables|/Script/Sclopetiator.VS_SclopetiatorGI|GetPistolStats _asgi_sclopetiator)))))
    (:then_2
      (Variables|Default|SetFireCooldownTime 0.1))))

(event EventTick
  (params (DeltaSeconds :type Float%20%28single-precision%29)))

(event EventReload
  (bind _reload_speed (Variables|Default|GetReload%20Speed))
  ;[1 1 1] Reload Firearm with Max Ammo Value
  (if (Variables|Default|GetisNotReloading)
    (Variables|Default|SetisNotReloading false)
    (bind _output_get (Variables|Default|SetCurrent%20Ammo (Variables|Default|GetMax%20Ammo)))
    (Default|CallEonCurrentAmmoModified _output_get)
    (Utilities|Time|SetTimerbyEvent (EventDispatchers|CreateEvent :!event ResetReloadCooldown) _reload_speed)
    (Variables|Default|SetisNotOnCooldown false)
    (Utilities|Time|SetTimerbyEvent (EventDispatchers|CreateEvent :!event ResetFireCooldown) _reload_speed)
    (Audio|PlaySound2D "/Game/Sclopetiator/Assets/Audio/MetaSound/MS_PistolReload.MS_PistolReload" 1.0 1.0 0.0 0 0)
    (|CallParentFunction)))

(event EventFire
  ;[1 1 1] Fires Single Bullet Per Click
  (|CallParentFunction))

(event EventBaseGunSetup
  (bind _returnvalue (Game|GetPlayerController 0))
  ;[1 1 1] On Collision and after Firearm is attached to the Player, set Pistol Widget to Gun Widget and Display to Player.
  (|CallParentFunction)
  (bind _returnvalue_2 (UserInterface|CreateWidget "/Game/Sclopetiator/Blueprints/Widget_Blueprints/WBP_Pistol.WBP_Pistol_C" _returnvalue))
  (Variables|Default|SetGun%20Widget _returnvalue_2)
  (bind _asbp_first_person_player_controller (Utilities|Casting|CastToBP_FirstPersonPlayerController _returnvalue))
  (Default|DisplayFirearmWidget _asbp_first_person_player_controller)
  (Default|CallEonCurrentAmmoModified (Variables|Default|GetCurrent%20Ammo))
  (Variables|/Script/Engine.RotatingMovementComponent|SetRotationRate (Variables|Default|GetRotatingMovement) "0, 0, 0"))

(fn ConstructionScript
  ;[1 1 1] Setting Defaults
)